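; Player controller for the Lexicon game that steers a pitch cursor and sets the game mode's drawing state.
; Tick sets clamped pitch from either mouse height or W/S input scaled by cursor speed and game speed.
; Space or left mouse requests drawing, which looping measure-length timers block during deadzones.
; Holding ToggleWordBank expands the lexicon, reroutes W/S to scrolling through Switch macros, and suspends drawing via gates.
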(event `self.ReceiveBeginPlay`
  (bind _deadzonelength (`self.DeadzoneLength`))
  (bind _mesurelength (`/Game/DataLayer/BP_LexiconGameMode.MesureLength` (`/Game/FL_GeneralGetters.Get_LexiconGameMode`)))
  (`KismetSystemLibrary.K2_SetTimerDelegate` (delegate `StartDeadzone`) _mesurelength true (/ _deadzonelength -2.0))
  (`KismetSystemLibrary.K2_SetTimerDelegate` (delegate `EndDeadzone`) _mesurelength true (/ _deadzonelength 2.0)))

(event `Key|W`
  (params (Key :type "Key Structure"))
  (bind _targetpitch (`self.TargetPitch`))
  ;[0 0.3844 0.0642] Keyboard Based Cursor Input; "isPressed" used to get around fake "release" activation on level init
  (:`Pressed`
    (`self.Switch` :!label _label
      (:`Out1`
        (`/Engine/EditorBlueprintResources/StandardMacros.DoOnce` false :!label _label_2
          (:`Completed`
            (`|ExecutionSequence`
              (:`then_0`
                (`/Engine/EditorBlueprintResources/StandardMacros.IncrementFloat` _targetpitch :!label _label_3))
              (:`then_1`
                (goto _label_4 :!via `Reset`))))))
      (:`Out2`
        (`self.OnScrollLexicon` "Scroll_Up"))))
  (:`Released`
    (`/Engine/EditorBlueprintResources/StandardMacros.DoOnce` true :!label _label_4
      (:`Completed`
        (`|ExecutionSequence`
          (:`then_0`
            (`/Engine/EditorBlueprintResources/StandardMacros.DecrementFloat` _targetpitch :!label _label_5))
          (:`then_1`
            (goto _label_2 :!via `Reset`)))))))

(event `InputAction|ToggleWordBank`
  (params (Key :type "Key Structure"))
  (bind _returnvalue (`/Game/FL_GeneralGetters.Get_LexiconGameMode`))
  ;[0 0 1] Expand/Collapse Lexicon when shift is pressed
  (:`Pressed`
    (`self.OnLexiconToggled` true)
    (`|ExecutionSequence`
      (:`then_0`
        (goto _label :!via `2`))
      (:`then_1`
        (goto _label_7 :!via `2`))
      (:`then_2`
        (goto _label_10 :!via `Close`))
      (:`then_3`
        (goto _label_11 :!via `Close`))
      (:`then_4`
        (set `self.WantsToDraw` false :!label _label_6)
        (`/Game/DataLayer/BP_LexiconGameMode.SetIsDrawing` _returnvalue false))))
  (:`Released`
    (`self.OnLexiconToggled` false)
    (`|ExecutionSequence`
      (:`then_0`
        (goto _label :!via `1`))
      (:`then_1`
        (goto _label_7 :!via `1`))
      (:`then_2`
        (goto _label_10 :!via `Open`))
      (:`then_3`
        (goto _label_11 :!via `Open`)))))

(event `StartDeadzone`
  (set `self.CanDraw` false)
  (`/Game/DataLayer/BP_LexiconGameMode.SetIsDrawing` (`/Game/FL_GeneralGetters.Get_LexiconGameMode`) false))

(event `EndDeadzone`
  (set `self.CanDraw` true)
  (`/Game/DataLayer/BP_LexiconGameMode.SetIsDrawing` (`/Game/FL_GeneralGetters.Get_LexiconGameMode`) (and (`self.WantsToDraw`) (`self.CanDraw`))))

(event `Key|S`
  (params (Key :type "Key Structure"))
  ;[0 0.3844 0.0642] Keyboard Based Cursor Input; "isPressed" used to get around fake "release" activation on level init
  (:`Pressed`
    (`self.Switch` :!label _label_7
      (:`Out1`
        (`/Engine/EditorBlueprintResources/StandardMacros.DoOnce` false :!label _label_8
          (:`Completed`
            (`|ExecutionSequence`
              (:`then_0`
                (goto _label_5))
              (:`then_1`
                (goto _label_9 :!via `Reset`))))))
      (:`Out2`
        (`self.OnScrollLexicon` "Scroll_Down"))))
  (:`Released`
    (`/Engine/EditorBlueprintResources/StandardMacros.DoOnce` true :!label _label_9
      (:`Completed`
        (`|ExecutionSequence`
          (:`then_0`
            (goto _label_3))
          (:`then_1`
            (goto _label_8 :!via `Reset`)))))))

(event `Key|SpaceBar`
  (params (Key :type "Key Structure"))
  (:`Pressed`
    (`/Engine/EditorBlueprintResources/StandardMacros.Gate` false :!label _label_10
      (:`Exit`
        (set `self.WantsToDraw` true)
        (`/Game/DataLayer/BP_LexiconGameMode.SetIsDrawing` (`/Game/FL_GeneralGetters.Get_LexiconGameMode`) (and (`self.WantsToDraw`) (`self.CanDraw`))))))
  (:`Released`
    (`/Engine/EditorBlueprintResources/StandardMacros.Gate` false :!label _label_11
      (:`Exit`
        (goto _label_6)))))

(event `self.ReceiveTick`
  (params (DeltaSeconds :type "Float (single-precision)"))
  (bind _returnvalue (`/Game/FL_GeneralGetters.Get_LexiconGameMode`))
  (bind (_returnvalue_x _returnvalue_y) (`KismetMathLibrary.BreakVector2D` (`WidgetLayoutLibrary.GetViewportSize`)))
  (`/Game/DataLayer/BP_LexiconGameMode.SetCurrentPitch` _returnvalue (`KismetMathLibrary.FClamp` (select `bool` (`self.MouseControl`) :`false` (+ (`/Game/DataLayer/BP_LexiconGameMode.GetCurrentPitch` _returnvalue) (* (`self.PitchCursorSpeed`) (`self.TargetPitch`) DeltaSeconds (`/Game/DataLayer/BP_DiffuclitySettings.GameSpeed` (`/Game/Core/BP_LexiconGameInstance.Difficulty` (`/Game/FL_GeneralGetters.Get_LexiconGameInstance`))))) :`true` (* (- 1.0 (/ (`.LocationY` (`self.GetMousePosition`)) _returnvalue_y 1.0)) (`self.MouseSensitivity`))))))

(event `Key|LeftMouseButton`
  (params (Key :type "Key Structure"))
  (:`Pressed`
    (goto _label_10))
  (:`Released`
    (goto _label_11)))

(fn `UserConstructionScript`)