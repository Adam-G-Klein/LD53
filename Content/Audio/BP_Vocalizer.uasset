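; BP_Vocalizer plays non-spatial vocal sound effects that bracket a spoken word, built from head, looping body and tail sounds.
; StartWord plays the head one-shot and spawns the body loop at the same moment, keeping its audio component.
; StopWord plays the tail one-shot and stops that stored component.
; All three sounds share a single pitch multiplier variable.
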(event `StartWord`
  (`GameplayStatics.PlaySound2D` (`self.SFX_Word_Head`) 1.0 (`self.SFX_PitchMultiplier`) 0.0 null null)
  (bind _returnvalue (`GameplayStatics.SpawnSound2D` (`self.SFX_Word_Body_Loop_Start`) 1.0 (`self.SFX_PitchMultiplier`) 0.0 null)))

(event `StopWord`
  (`GameplayStatics.PlaySound2D` (`self.SFX_Word_Tail`) 1.0 (`self.SFX_PitchMultiplier`) 0.0 null null)
  (`AudioComponent.Stop` (stale `StartWord` _returnvalue)))

(fn `UserConstructionScript`)