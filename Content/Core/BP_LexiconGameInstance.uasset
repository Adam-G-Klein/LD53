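; Game instance for Lexicon that owns level progression and its persistence through a BP_ProgressSaveGame.
; On Init it loads the progress slot, or creates a fresh save object if that fails.
; DT_LevelGoals row names double as map names, indexed by the saved current level to open levels.
; Level changes save asynchronously, and an out-of-range index returns to the main menu and resets progress to zero.
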(event `self.ReceiveInit`
  (bind _progesssaveslotname (`self.ProgessSaveSlotName`))
  ;[1 1 1] Load Current Progress
  (bind _returnvalue (`GameplayStatics.DoesSaveGameExist` _progesssaveslotname))
  (if _returnvalue
    (bind _returnvalue_2 (`GameplayStatics.LoadGameFromSlot` _progesssaveslotname))
    (bind _asbp_progress_save_game (cast `/Game/Core/BP_ProgressSaveGame` _returnvalue_2)
      (:`then`
        (set `self.ProgressSaveGame` _asbp_progress_save_game))
      (:`CastFailed`
        (bind _returnvalue_3 (`|GenericCreateObject` "/Game/Core/BP_ProgressSaveGame.BP_ProgressSaveGame_C" :!label _label))
        (set `self.ProgressSaveGame` _returnvalue_3)))
    (else
      (goto _label))))

(event `ResetProgress`
  (params (OpenLevel :type Boolean))
  (if OpenLevel
    (`self.OpenLevel` 0)
    (else
      (set `/Game/Core/BP_ProgressSaveGame.CurrentLevelIndex` 0 (`self.ProgressSaveGame`))
      (`AsyncActionHandleSaveGame.AsyncSaveGameToSlot` self (`self.ProgressSaveGame`) (`self.ProgessSaveSlotName`)))))

(event `OpenCurrentLevel`
  (bind (_returnvalue _levelname) (`self.GetCurrentLevel`))
  ;[1 1 1] Level Opening
  (if _returnvalue
    (`GameplayStatics.OpenLevel` _levelname)
    (else
      (`self.OpenMainMenu`)
      (set `/Game/Core/BP_ProgressSaveGame.CurrentLevelIndex` 0 (`self.ProgressSaveGame`))
      (`AsyncActionHandleSaveGame.AsyncSaveGameToSlot` self (`self.ProgressSaveGame`) (`self.ProgessSaveSlotName`)))))

(event `OpenNextLevel`
  ;[1 1 1] Level Opening
  (`/Engine/EditorBlueprintResources/StandardMacros.IncrementInt` (`/Game/Core/BP_ProgressSaveGame.CurrentLevelIndex` (`self.ProgressSaveGame`))
    (:`  `
      (`self.OpenCurrentLevel`)
      (`AsyncActionHandleSaveGame.AsyncSaveGameToSlot` self (`self.ProgressSaveGame`) (`self.ProgessSaveSlotName`)))))

(event `OpenLevel`
  (params (Level :type Integer))
  ;[1 1 1] Level Opening
  (set `/Game/Core/BP_ProgressSaveGame.CurrentLevelIndex` Level (`self.ProgressSaveGame`))
  (`self.OpenCurrentLevel`)
  (`AsyncActionHandleSaveGame.AsyncSaveGameToSlot` self (`self.ProgressSaveGame`) (`self.ProgessSaveSlotName`)))

(event `OpenMainMenu`
  ;[1 1 1] Level Opening
  (`GameplayStatics.OpenLevelBySoftObjectPtr` "/Game/Maps/MainMenuMap.MainMenuMap"))

(fn `GetCurrentLevel`
  (returns (ReturnValue :type Boolean) (LevelName :type Name) (Index :type Integer))
  (bind _currentlevelindex (`/Game/Core/BP_ProgressSaveGame.CurrentLevelIndex` (`self.ProgressSaveGame`)))
  (bind _outrownames (`DataTableFunctionLibrary.GetDataTableRowNames` "/Game/Core/DT_LevelGoals.DT_LevelGoals"))
  (return (`KismetArrayLibrary.Array_IsValidIndex` _outrownames _currentlevelindex) (`|GetArrayItem` _outrownames _currentlevelindex) _currentlevelindex))