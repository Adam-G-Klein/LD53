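; Game mode that records the player's drawn pitch-over-time curves into measures and creates the HUD and dialog widgets.
; Tick advances time by the difficulty game speed, starting a new measure each measure length and duplicating the last key at each key interval while drawing.
; Pitch and time setters stretch the live last key and curve end.
; Dispatchers announce new measures, curves and keys, plus curve ends.
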(event `self.ReceiveTick`
  (params (DeltaSeconds :type "Float (single-precision)"))
  (bind _currenpitch (`self.GetCurrentPitch`))
  (bind _measures (`self.Measures`))
  (bind _output_curves (break `/Game/DataLayer/F_Measure` (`|GetArrayItem` _measures (`KismetArrayLibrary.Array_LastIndex` _measures))))
  (bind _returnvalue (* DeltaSeconds (`/Game/DataLayer/BP_DiffuclitySettings.GameSpeed` (`/Game/Core/BP_LexiconGameInstance.Difficulty` (`/Game/FL_GeneralGetters.Get_LexiconGameInstance`)))))
  (bind (_output_start _output_end _output_keys) (break `/Game/DataLayer/F_Curve` (`|GetArrayItem` _output_curves (`KismetArrayLibrary.Array_LastIndex` _output_curves))))
  (bind _returnvalue_2 (+ _returnvalue (`self.CurrentTime`)))
  (`|ExecutionSequence`
    (:`then_0`
      ;[1 1 1] New Mesures
      (if (<= (mod _returnvalue_2 (`self.MesureLength`)) _returnvalue)
        (`|ExecutionSequence`
          (:`then_0`
            (if (`self.IsDrawing`)
              (`KismetArrayLibrary.Array_Add` (`self.Measures`) (make `/Game/DataLayer/F_Measure` (`|MakeArray` (make `/Game/DataLayer/F_Curve` 0.0 (mod (`self.CurrentTime`) (`self.MesureLength`)) (`|MakeArray` (make `/Game/DataLayer/F_CurveKey` 0.0 _currenpitch) (make `/Game/DataLayer/F_CurveKey` (mod (`self.CurrentTime`) (`self.MesureLength`)) _currenpitch) :!type "/Game/DataLayer/F_CurveKey Structure")) :!type "/Game/DataLayer/F_Curve Structure")))
              (`self.OnNewCurveCreated`)
              (else
                (`KismetArrayLibrary.Array_Add` (`self.Measures`)) ; What if player doesn't hold drawing down until the end of the measure?\nWe should probably still add the curve in that case is possible
              )))
          (:`then_1`
            (`self.NewMeasureStarted`)))
        (else
          ;[1 1 1] New Keys
          (if (and (<= (mod _returnvalue_2 (`self.KeyInterval`)) _returnvalue) (`self.IsDrawing`))
            (`KismetArrayLibrary.Array_Add` _output_keys (`|GetArrayItem` _output_keys (`KismetArrayLibrary.Array_LastIndex` _output_keys)))
            (`self.OnKeyAddedToCurrentCurve`)))))
    (:`then_1`
      (`self.SetCurrentTime` _returnvalue_2))))

(event `self.ReceiveBeginPlay`
  ;[0 0 1] Create the HUD, display on screen
  (bind _returnvalue (`|CreateWidget` "/Game/UI/WBP_HUD.WBP_HUD_C"))
  (`UserWidget.AddToViewport` _returnvalue 0)
  (bind _returnvalue_2 (`|CreateWidget` "/Game/UI/WBP_Dialog.WBP_Dialog_C"))
  (`UserWidget.AddToViewport` _returnvalue_2 0))

(fn `GetCurrentPitch`
  (returns (CurrenPitch :type "Float (double-precision)"))
  (return (`self.CurrenPitch`)))

(fn `GetCurrentTime`
  (returns (CurrentTime :type "Float (double-precision)"))
  (return (`self.CurrentTime`)))

(fn `GetIsDrawing`
  (returns (IsDrawing :type Boolean))
  (return (`self.IsDrawing`)))

(fn `GetMesures`
  (returns (Measures :type "Array of /Game/DataLayer/F_Measure Structure"))
  (return (`self.Measures`)))

(fn `SetCurrentPitch`
  (params (CurrentPitch :type "Float (double-precision)"))
  (bind _measures (`self.Measures`))
  (bind _output_curves (break `/Game/DataLayer/F_Measure` (`|GetArrayItem` _measures (`KismetArrayLibrary.Array_LastIndex` _measures))))
  (bind (_start _end _keys) (break `/Game/DataLayer/F_Curve` (`|GetArrayItem` _output_curves (`KismetArrayLibrary.Array_LastIndex` _output_curves))))
  (set `self.CurrenPitch` CurrentPitch)
  (if (`self.IsDrawing`)
    (setmembers `/Game/DataLayer/F_CurveKey` :`StructRef` (`|GetArrayItem` _keys (`KismetArrayLibrary.Array_LastIndex` _keys)) :`Pitch` (`self.CurrenPitch`))))

(fn `SetCurrentTime`
  (params (CurrentTime :type "Float (double-precision)"))
  (locals (Keys :type "Array of /Game/DataLayer/F_CurveKey Structure"))
  (bind _measures (`self.Measures`))
  (bind _returnvalue (mod (`self.GetCurrentTime`) (`self.MesureLength`)))
  (bind _output_curves (break `/Game/DataLayer/F_Measure` (`|GetArrayItem` _measures (`KismetArrayLibrary.Array_LastIndex` _measures))))
  (bind _output (`|GetArrayItem` _output_curves (`KismetArrayLibrary.Array_LastIndex` _output_curves)))
  (bind (_start _end _keys) (break `/Game/DataLayer/F_Curve` _output))
  (set `self.CurrentTime` CurrentTime)
  (if (`self.GetIsDrawing`)
    (setmembers `/Game/DataLayer/F_CurveKey` :`StructRef` (`|GetArrayItem` _keys (`KismetArrayLibrary.Array_LastIndex` _keys)) :`Time` _returnvalue)
    (setmembers `/Game/DataLayer/F_Curve` :`StructRef` _output :`End` _returnvalue)))

(fn `SetIsDrawing`
  (params (IsDrawing :type Boolean))
  (bind _currenpitch (`self.GetCurrentPitch`))
  (bind _measures (`self.Measures`))
  (bind _returnvalue (mod (`self.GetCurrentTime`) (`self.MesureLength`)))
  (bind _output_curves (break `/Game/DataLayer/F_Measure` (`|GetArrayItem` _measures (`KismetArrayLibrary.Array_LastIndex` _measures))))
  (`|ExecutionSequence`
    (:`then_0`
      (if (and IsDrawing (not (`self.IsDrawing`)))
        (`KismetArrayLibrary.Array_Add` _output_curves (make `/Game/DataLayer/F_Curve` _returnvalue _returnvalue (`|MakeArray` (make `/Game/DataLayer/F_CurveKey` _returnvalue _currenpitch) (make `/Game/DataLayer/F_CurveKey` _returnvalue _currenpitch) :!type "/Game/DataLayer/F_CurveKey Structure")))
        (`self.OnNewCurveCreated`)
        (elif (and (`self.IsDrawing`) (not IsDrawing))
          (`self.OnCurveEnded`))))
    (:`then_1`
      (set `self.IsDrawing` IsDrawing))))

(fn `UserConstructionScript`)