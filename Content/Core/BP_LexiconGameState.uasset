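; Game state for the Lexicon drawing word game, holding lives, score and the current goal word index.
; BeginPlay takes lives from game mode difficulty, then waits for the first curve before binding to new-measure events.
; Goal words resolve from the level's DT_LevelGoals row into DT_Words entries.
; ScoreLatestMesure currently only prints the second-to-last measure's similarity to "ToWant"; closest-word scoring, life loss and win/lose logic are disconnected.
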(event `self.ReceiveBeginPlay`
  ;[1 1 1] InitalizeLives
  (set `self.Lives` (`/Game/DataLayer/BP_DiffuclitySettings.Lives` (`/Game/DataLayer/BP_LexiconGameMode.CurrentDifficulty` (`/Game/FL_GeneralGetters.Get_LexiconGameMode`))))
  ;[1 1 1] Wait for drawing to start before scoring
  (add `/Game/DataLayer/BP_LexiconGameMode.OnNewCurveCreated` (`/Game/FL_GeneralGetters.Get_LexiconGameMode`) (delegate `DrawingStarted`)))

(event `DrawingStarted`
  (bind _returnvalue (`/Game/FL_GeneralGetters.Get_LexiconGameMode`))
  ;[1 1 1] Wait for drawing to start before scoring
  (remove `/Game/DataLayer/BP_LexiconGameMode.OnNewCurveCreated` _returnvalue (delegate `DrawingStarted`))
  (add `/Game/DataLayer/BP_LexiconGameMode.NewMeasureStarted` _returnvalue (`|CreateDelegate` :!event `ScoreLatestMesure`)))

(fn `GetCurrentGoalWord`
  (returns (EnglishWord :type String))
  (bind _goalwords (`self.GetCurrentGoalWords`))
  (return (`.EnglishWord_2_0BA26D0741784E2A3DD542A290E8226D` (break `/Game/DataLayer/F_WordObject` (`|GetArrayItem` _goalwords (`self.CurrentGoalWordIndex`))))))

(fn `GetCurrentGoalWordIndex`
  (returns (ReturnValue :type Integer))
  (return (`self.CurrentGoalWordIndex`)))

(fn `GetCurrentGoalWords`
  (returns (GoalWords :type "Array of /Game/DataLayer/F_WordObject Structure"))
  (locals (CurrentGoalWords :type "Array of /Game/DataLayer/F_WordObject Structure"))
  ;[0 0 1] Get the current level's goal words
  (bind _returnvalue (`|GetDataTableRow` "/Game/Core/DT_LevelGoals.DT_LevelGoals" (`.LevelName` (`/Game/Core/BP_LexiconGameInstance.GetCurrentLevel` (`/Game/FL_GeneralGetters.Get_LexiconGameInstance`))))
    (:`then`
      ;[0 0 1] Create an Array<FWordObject> to return from the list of goal words
      (for _array_element (`.GoalWords_7_F5980C9344F1C9942C4B8DA4DC2D03E2` (break `/Game/Core/F_LevelGoal` _returnvalue))
        (bind _returnvalue_2 (`|GetDataTableRow` "/Game/DataLayer/DT_Words.DT_Words" (`.RowName` (break `DataTableRowHandle` _array_element)))
          (:`then`
            (`KismetArrayLibrary.Array_Add` (`local.CurrentGoalWords`) _returnvalue_2)))))
    (:`RowNotFound`
      _))
  (return (`local.CurrentGoalWords`)))

(fn `GetLives`
  (returns (ReturnValue :type Integer))
  (return (`self.Lives`)))

(fn `GetScore`
  (returns (ReturnValue :type Integer))
  (return (`self.Score`)))

(fn `ScoreLatestMesure`
  (locals (CurrentGoalWords :type "Array of /Game/DataLayer/F_WordObject Structure"))
  (bind _measures (`/Game/DataLayer/BP_LexiconGameMode.GetMesures` (`/Game/FL_GeneralGetters.Get_LexiconGameMode`)))
  (bind _goalwords (`self.GetCurrentGoalWords`))
  (set `local.CurrentGoalWords` _goalwords)
  (bind _returnvalue (`|GetDataTableRow` "/Game/DataLayer/DT_Words.DT_Words" "ToWant")
    (:`then`
      (`KismetSystemLibrary.PrintString` (`KismetStringLibrary.Conv_DoubleToString` (`/Game/DataLayer/FL_MesureUtilites.GetMeasureSimilarity` (`.SansSerifGlyphMeasure_14_04C174124059B23CFF094FA35C52EEA0` (break `/Game/DataLayer/F_WordObject` _returnvalue)) (`|GetArrayItem` _measures (- (`KismetArrayLibrary.Array_LastIndex` _measures) 1))))))))

(fn `UserConstructionScript`)