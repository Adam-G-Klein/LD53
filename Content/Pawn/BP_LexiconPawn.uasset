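; Pawn that visualizes the Lexicon game mode's pitch curves as a scrolling trail drawn by a cursor.
; Each Tick sets cursor height from current pitch and scrolls the camera with current time.
; Game mode curve events toggle the cursor sprite and start or release spline mesh segments.
; The active segment's end follows the cursor with a tangent along its direction, while segments older than a threshold are destroyed.
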(event `self.ReceiveBeginPlay`
  (bind _returnvalue (`/Game/FL_GeneralGetters.Get_LexiconGameMode`))
  ;[1 1 1] Event Handling
  (add `/Game/DataLayer/BP_LexiconGameMode.OnKeyAddedToCurrentCurve` _returnvalue (`|CreateDelegate` :!event `CreateNewSpline`))
  (add `/Game/DataLayer/BP_LexiconGameMode.OnNewCurveCreated` _returnvalue (delegate `CurveStarted`))
  (add `/Game/DataLayer/BP_LexiconGameMode.OnCurveEnded` _returnvalue (delegate `CurveEnded`)))

(event `CurveEnded`
  ;[1 1 1] Event Handling
  (set `self.CurrentSpline` null)
  (`PaperSpriteComponent.SetSprite` (`self.S_Cursor`) "/Game/Pawn/S_CURSOR_OFF_FINAL.S_CURSOR_OFF_FINAL"))

(event `CurveStarted`
  ;[1 1 1] Event Handling
  (`PaperSpriteComponent.SetSprite` (`self.S_Cursor`) "/Game/Pawn/S_CURSOR_ON_FINAL.S_CURSOR_ON_FINAL")
  (`self.CreateNewSpline`))

(event `self.ReceiveTick`
  (params (DeltaSeconds :type "Float (single-precision)"))
  (bind _returnvalue (`self.K2_GetComponentsByClass` "/Script/Engine.SplineMeshComponent"))
  (bind _returnvalue_x (`KismetMathLibrary.BreakVector` (`self.CursorWorldSpaceLocation`)))
  (bind _currentspline (`self.CurrentSpline`))
  (bind _s_cursor (`self.S_Cursor`))
  (bind (_returnvalue_x_2 _returnvalue_y _returnvalue_z) (`KismetMathLibrary.BreakVector` (`SceneComponent.K2_GetComponentLocation` (`self.Camera`))))
  (bind _output (`|GetArrayItem` _returnvalue))
  (bind (_relativelocation_x _relativelocation_y _relativelocation_z) (`KismetMathLibrary.BreakVector` (`SceneComponent.RelativeLocation` _s_cursor)))
  (bind (_relativescale3d_x _relativescale3d_y) (`KismetMathLibrary.BreakVector` (`SceneComponent.RelativeScale3D` _s_cursor)))
  (bind _returnvalue_x_3 (`KismetMathLibrary.BreakVector` (`SplineMeshComponent.GetStartPosition` _output)))
  ;[1 1 1] Move Cursor
  (`SceneComponent.K2_SetRelativeLocation` _s_cursor (`KismetMathLibrary.MakeVector` 0.0 (* (- 0.5 (`/Game/DataLayer/BP_LexiconGameMode.GetCurrentPitch` (`/Game/FL_GeneralGetters.Get_LexiconGameMode`))) (`self.PitchHeight`) _relativescale3d_y) _relativelocation_z) false false)
  ;[1 1 1] Scroll Camera
  (`SceneComponent.K2_SetRelativeLocation` (`self.Camera`) (`KismetMathLibrary.MakeVector` (* (`/Game/DataLayer/BP_LexiconGameMode.GetCurrentTime` (`/Game/FL_GeneralGetters.Get_LexiconGameMode`)) (`self.SecondLength`)) 0.0 _returnvalue_z) false false)
  (`|ExecutionSequence`
    (:`then_0`
      ;[1 1 1] Update Current Spline
      (bind _currentspline_2 (`self.CurrentSpline`)
        (:`then`
          (bind _output_get (set `self.CurrentTangent` (`KismetMathLibrary.Normal2D` (`KismetMathLibrary.Conv_VectorToVector2D` (- (`self.CursorWorldSpaceLocation`) (`SplineMeshComponent.GetEndPosition` _currentspline_2))))))
          (`SplineMeshComponent.SetEndTangent` _currentspline (* (`KismetMathLibrary.Conv_Vector2DToVector` _output_get) (`self.TangentLength`)) false)
          (`SplineMeshComponent.SetEndPosition` _currentspline (`self.CursorWorldSpaceLocation`) true))
        (:`else`)))
    (:`then_1`
      ;[1 1 1] Kill Old Splines
      (if (`KismetArrayLibrary.Array_IsNotEmpty` _returnvalue)
        (`/Engine/EditorBlueprintResources/StandardMacros.IsValid` _output
          (:`Is Valid`
            (if (> (- _returnvalue_x _returnvalue_x_3) (* (`self.KillCurvesOlderThan`) (`self.SecondLength`)))
              (`ActorComponent.K2_DestroyComponent` _output))))))))

(fn `CreateNewSpline`
  (bind _returnvalue (`self.CursorWorldSpaceLocation`))
  (bind _tangentlength (`self.TangentLength`))
  (bind _returnvalue_2 (`KismetMathLibrary.Conv_Vector2DToVector` (* (`self.CurrentTangent`) (`KismetMathLibrary.MakeVector2D` _tangentlength _tangentlength))))
  (bind _returnvalue_3 (`AddComponent|NODE_AddSplineMeshComponent-1` :`RelativeTransform` (`KismetMathLibrary.MakeTransform` (`KismetMathLibrary.MakeVector` 0.0 (`self.YOffest`)))))
  (bind _output_get (set `self.CurrentSpline` _returnvalue_3))
  (`SplineMeshComponent.SetStartAndEnd` _output_get _returnvalue _returnvalue_2 _returnvalue _returnvalue_2 true))

(fn `CursorWorldSpaceLocation`
  (returns (ReturnValue :type "Vector Structure"))
  (bind _returnvalue (`/Game/FL_GeneralGetters.Get_LexiconGameMode`))
  (return (`KismetMathLibrary.MakeVector` (* (`/Game/DataLayer/BP_LexiconGameMode.GetCurrentTime` _returnvalue) (`self.SecondLength`)) (* (- (`/Game/DataLayer/BP_LexiconGameMode.GetCurrentPitch` _returnvalue) 0.5) (`self.PitchHeight`)))))

(fn `UserConstructionScript`
  (`self.K2_SetActorLocationAndRotation` (0.0 0.0 0.0)))