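; Emoji VFX spawner actor that plays one of seven Niagara emoji effects, such as whale, taco or banana.
; SpawnEmojis maps EmojiNum to a system and spawns it attached to the VFXEmitter component at the LocationToSpawn relative offset.
; An EmojiNum of zero picks a random effect by rolling a new number and calling the event again, overwriting the stored value.
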(event `SpawnEmojis`
  (switch `int` (`self.EmojiNum`)
    (:`0`
      (set `self.EmojiNum` (`KismetMathLibrary.RandomIntegerInRange` 1 7))
      (`self.SpawnEmojis`))
    (:`1`
      (set `self.ChosenNS` (`self.Whale`))
      (`NiagaraFunctionLibrary.SpawnSystemAttached` (`self.ChosenNS`) (`self.VFXEmitter`) "None" (`self.LocationToSpawn`) (struct) "KeepRelativeOffset" :!label _label))
    (:`2`
      (set `self.ChosenNS` (`self.Taco`))
      (goto _label))
    (:`3`
      (set `self.ChosenNS` (`self.Gem`))
      (goto _label))
    (:`4`
      (set `self.ChosenNS` (`self.Cactus`))
      (goto _label))
    (:`5`
      (set `self.ChosenNS` (`self.Yarn`))
      (goto _label))
    (:`6`
      (set `self.ChosenNS` (`self.Lightning`))
      (goto _label))
    (:`7`
      (set `self.ChosenNS` (`self.Banana`))
      (goto _label))))

(fn `UserConstructionScript`)