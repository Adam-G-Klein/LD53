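; BP_GetCurveDataExample is a reference Blueprint showing how to access pitch curve data on the Lexicon game mode.
; Unconnected node snippets read curve keys (X is time, Y is pitch) from Dictionary entries and Measures, plus current time and pitch.
; Others show setting the current pitch and appending a measure.
; Nothing is wired to an event, so none of it executes.
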(fn `UserConstructionScript`)